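; BP_Dissolvenza3 is a dissolve actor that drives a material effect on cube and metal fence meshes when the player character enters its trigger.
; On BeginPlay it applies one shared dynamic instance of M_Disoolvenza1 to all six meshes.
; Overlapping CollisioneDissolvenza plays the Dissolvenza timeline, which feeds the QuantitaDissolvenza scalar parameter.
; Leaving reverses the timeline from its end, even if playback was incomplete.
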(event OnComponentBeginOverlap(CollisioneDissolvenza)
  (params (OverlappedComponent :type Primitive%20Component%20Object%20Reference) (OtherActor :type Actor%20Object%20Reference) (OtherComp :type Primitive%20Component%20Object%20Reference) (OtherBodyIndex :type Integer) (bFromSweep :type Boolean) (SweepResult :type Hit%20Result%20Structure%20%28by%20ref%29))
  (Utilities|Casting|CastToBP_ThirdPersonCharacter OtherActor)
  (bind _dissolvenza (Timeline|Dissolvenza Play)
    (:Update
      (Rendering|Material|SetScalarParameterValue (Variables|Default|GetCrea%20Dissolvenza) "QuantitaDissolvenza" _dissolvenza :!class /Script/Engine.MaterialInstanceDynamic))))

(event OnComponentEndOverlap(CollisioneDissolvenza)
  (params (OverlappedComponent :type Primitive%20Component%20Object%20Reference) (OtherActor :type Actor%20Object%20Reference) (OtherComp :type Primitive%20Component%20Object%20Reference) (OtherBodyIndex :type Integer))
  (Utilities|Casting|CastToBP_ThirdPersonCharacter OtherActor)
  (bind _dissolvenza (Timeline|Dissolvenza ReverseFromEnd)
    (:Update
      (Rendering|Material|SetScalarParameterValue (Variables|Default|GetCrea%20Dissolvenza) "QuantitaDissolvenza" _dissolvenza :!class /Script/Engine.MaterialInstanceDynamic))))

(event EventBeginPlay
  (bind _returnvalue (Rendering|Material|CreateDynamicMaterialInstance "/Game/Materials/M_Disoolvenza1.M_Disoolvenza1" "" "None" :!class /Script/Engine.KismetMaterialLibrary))
  (bind _output_get (Variables|Default|SetCrea%20Dissolvenza _returnvalue))
  (Rendering|Material|SetMaterial (Variables|Default|GetCube4) 0 _output_get))

(fn ConstructionScript)