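; BP_CatapultaAVANTIvELOCITAfOLLE1 is a catapult pad that launches the third-person player character along a configurable direction.
; When the character overlaps its Box, it calls LaunchCharacter with a velocity built from the ArrowVector's up and forward vectors.
; Each axis has its own weight and Speed scales the sum, which adds to the character's current velocity instead of overriding it.
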(event OnComponentBeginOverlap(Box)
  (params (OverlappedComponent :type Primitive%20Component%20Object%20Reference) (OtherActor :type Actor%20Object%20Reference) (OtherComp :type Primitive%20Component%20Object%20Reference) (OtherBodyIndex :type Integer) (bFromSweep :type Boolean) (SweepResult :type Hit%20Result%20Structure%20%28by%20ref%29))
  (bind _asbp_third_person_character (Utilities|Casting|CastToBP_ThirdPersonCharacter OtherActor))
  (Character|LaunchCharacter _asbp_third_person_character (* (Variables|Default|GetSpeed) (+ (* (Math|Vector|GetUpVector (Variables|Default|GetArrowVector)) (Variables|Default|GetVelocitaUP)) (* (Math|Vector|GetForwardVector (Variables|Default|GetArrowVector)) (Variables|Default|GetVelocitaAVANTI)))) false false))

(event EventBeginPlay)

(event Collision|EventActorBeginOverlap
  (params (OtherActor :type Actor%20Object%20Reference)))

(event EventTick
  (params (DeltaSeconds :type Float%20%28single-precision%29)))

(fn ConstructionScript)